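; BP_Monster is an AI monster actor that can be stunned, with Stun currently destroying it immediately.
; BeginPlay caches the player character, and Tick plays the Stun montage whenever IsStunned is true, then sets a Blackboard bool and destroys the actor after a delay.
; The timed stun/unstun and chase-binding logic is disconnected, and AttackPlayer is an empty stub.
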(event EventBeginPlay
  (bind _asbp_player_character (Utilities|Casting|CastToBP_PlayerCharacter (Game|GetPlayerCharacter 0))))

(event Collision|EventActorBeginOverlap
  (params (OtherActor :type Actor%20Object%20Reference)))

(event EventTick
  (params (DeltaSeconds :type Float%20%28single-precision%29))
  (if (Variables|Default|GetisStunned)
    (Animation|Montage|PlayMontage 0 "/Game/Animation/Zombie/AM_Monster.AM_Monster" 1.0 0.0 "Stun"
      (:OnCompleted
        (AI|Components|Blackboard|SetValueasBool (AI|GetBlackboard (AI|GetAIController self)) (Variables|Default|GetKey) true)
        (Utilities|FlowControl|Delay 3.0)
        (Actor|DestroyActor)))))

(fn ConstructionScript)

(fn Stun
  (Actor|DestroyActor))

(fn Unstun
  (Variables|Default|SetisStunned false))

(fn AttackPlayer)