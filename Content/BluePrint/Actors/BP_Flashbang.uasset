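; BP_Flashbang is a thrown projectile actor that detonates on a short fixed timer.
; On BeginPlay it launches ProjectileMovement with InitialVelocity, then enables blocking collision on its mesh after a brief delay.
; After a second delay it turns on physics simulation and immediately spawns BP_Explosion at its location, then destroys itself.
; The Explode function is an empty stub, and no flash effect is implemented in this Blueprint.
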(event EventBeginPlay
  (bind _projectilemovement (Variables|Default|GetProjectileMovement))
  (Variables|/Script/Engine.MovementComponent|SetVelocity _projectilemovement (Variables|Default|GetInitial%20Velocity))
  (Components|Activation|Activate _projectilemovement false)
  (Utilities|FlowControl|Delay 0.2)
  (Collision|SetCollisionProfileName (Variables|Default|GetStaticMesh) "BlockAllDynamic" true :!class /Script/Engine.PrimitiveComponent)
  (Utilities|FlowControl|Delay 0.2)
  (Physics|SetSimulatePhysics (Variables|Default|GetStaticMesh) true)
  (Game|SpawnActorfromClass "/Game/BluePrint/BP_Explosion.BP_Explosion_C" (Math|Conversions|ToTransform(Vector) (Transformation|GetActorLocation)) "Undefined" "MultiplyWithRoot" 0 0)
  (Actor|DestroyActor))

(event Collision|EventActorBeginOverlap
  (params (OtherActor :type Actor%20Object%20Reference)))

(event EventTick
  (params (DeltaSeconds :type Float%20%28single-precision%29)))

(fn ConstructionScript)

(fn Explode)