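; BP_LightCheckComponent is an unfinished light-check component, apparently meant to detect nearby spot lights.
; It schedules CheckLight at CheckInterval twice over, through a looping timer from BeginPlay and an elapsed-time accumulator in Tick.
; CheckLight is empty: its sphere overlap query for SpotLight actors within LightCheckRadius is unconnected, so the checks currently do nothing.
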(event EventBeginPlay
  (Utilities|Time|SetTimerbyFunctionName 0 "CheckLight" (Variables|Default|GetCheckInterval) true))

(event EventTick
  (params (DeltaSeconds :type Float%20%28single-precision%29))
  (bind _output_get (Variables|Default|Set_TimeSinceLastCheck (+ DeltaSeconds (Variables|Default|Get_TimeSinceLastCheck))))
  (if (>= _output_get (Variables|Default|GetCheckInterval))
    (Variables|Default|Set_TimeSinceLastCheck 0.0)
    (CallFunction|CheckLight)))

(fn CheckLight)