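; BP_Explosion is a short-lived expanding blast actor that stuns monsters it touches.
; Each tick it grows the actor scale by GrowthRate over delta time, then destroys itself once one second has elapsed.
; It also resets Sphere1's radius every tick to the initial radius times that frame's growth step, without accumulating.
; Sphere1's begin overlap calls Stun on BP_Monster actors; a BP_Monster_nonAI branch is left unconnected.
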(event OnComponentBeginOverlap(Sphere1)
  (params (OverlappedComponent :type Primitive%20Component%20Object%20Reference) (OtherActor :type Actor%20Object%20Reference) (OtherComp :type Primitive%20Component%20Object%20Reference) (OtherBodyIndex :type Integer) (bFromSweep :type Boolean) (SweepResult :type Hit%20Result%20Structure%20%28by%20ref%29))
  (bind _asbp_monster (Utilities|Casting|CastToBP_Monster OtherActor))
  (Default|Stun _asbp_monster))

(event EventBeginPlay
  (Variables|Default|SetNewRadius (Class|SphereComponent|GetUnscaledSphereRadius (Variables|Default|GetSphere1))))

(event Collision|EventActorBeginOverlap
  (params (OtherActor :type Actor%20Object%20Reference)))

(event EventTick
  (params (DeltaSeconds :type Float%20%28single-precision%29))
  (bind _output_get (Variables|Default|SetElapsedTime (+ DeltaSeconds (Variables|Default|GetElapsedTime))))
  (if (>= _output_get 1.0)
    (Actor|DestroyActor)
    (else
      (Transformation|SetActorScale3D (+ (* DeltaSeconds (Variables|Default|GetGrowthRate)) (Transformation|GetActorScale3D)))
      (Components|Sphere|SetSphereRadius (Variables|Default|GetSphere1) (* (Variables|Default|GetNewRadius) (* DeltaSeconds (Variables|Default|GetGrowthRate))) true))))

(fn ConstructionScript)